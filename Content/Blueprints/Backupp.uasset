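; Scratch Blueprint named Backupp that tests hit-indicator angle math on an F key press.
; The key runs the SHOWALLSCREENMESSAGES console command, then prints a yaw difference and "Hello".
; The yaw difference compares a negated, flattened direction with the actor's flattened forward vector, but the direction input is a hardcoded zero vector.
; All other events and the construction script are empty.
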(event EventBeginPlay
  ;[1 1 1] Hit Indicator
)

(event Collision|EventActorBeginOverlap
  (params (OtherActor :type Actor%20Object%20Reference))
  ;[1 1 1] Hit Indicator
)

(event EventTick
  (params (DeltaSeconds :type Float%20%28single-precision%29)))

(event Input|KeyboardEvents|F
  (params (Key :type Key%20Structure))
  (:Pressed
    (Development|ExecuteConsoleCommand "SHOWALLSCREENMESSAGES" 0)
    ;[1 1 1] Hit Indicator
    (Development|PrintString (Utilities|String|ToString(Float) (- (.Yaw (Math|Rotator|BreakRotator (Math|Conversions|RotationFromXVector (Math|Vector|Normalize (* (Math|Vector|MakeVector 0.0 0.0 0.0) "-1.000000,-1.000000,0.000000"))))) (.Yaw (Math|Rotator|BreakRotator (Math|Conversions|RotationFromXVector (Math|Vector|Normalize (* (Transformation|GetActorForwardVector) "1.000000,1.000000, 0"))))))))
    (Development|PrintString "Hello")))

(fn ConstructionScript)