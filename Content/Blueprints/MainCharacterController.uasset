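; Player ship Blueprint with a cockpit, handling shooting sound, shield spawning, damage feedback and a resource orb drop on death.
; BP-suffixed events act as cosmetic and spawn hooks, including camera shake and opening or closing the ability menu.
; BeginPlay creates that menu for the local player and strips cockpit components from other players' ships.
; Timelines drive damage and shield vignettes through a Material Parameter Collection, and keys swap Raptor and Cow cockpit props.
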(event Custom|ScreenShake
  (Class|PlayerController|ClientPlayCameraShake (Game|GetPlayerController 0) "/Game/Blueprints/CameraShake01.CameraShake01_C" 1.0 "CameraLocal" "0, 0, 0"))

(event Custom|BroadcastPlaySound
  (Audio|SpawnSoundAttached "/Game/Audio/FX/ShipFXShoot01_Cue.ShipFXShoot01_Cue" (Variables|Default|GetCollider) "None" "0, 0, 0" "0, 0, 0" "KeepRelativeOffset" false 1.0 1.0 0.0 0 0))

(event Custom|PlayPP
  ;[1 1 1] Enable Shield Vignete
  (bind (_direction _vigneteopacity _vignetteradius) (Timeline|Timeline_1 PlayFromStart)
    (:Update
      (Rendering|Material|SetScalarParameterValue "/Game/Materials/PlayerFX_Collection.PlayerFX_Collection" "DamageVignetteOpacity" _vigneteopacity :!class /Script/Engine.KismetMaterialLibrary)
      (Rendering|Material|SetScalarParameterValue "/Game/Materials/PlayerFX_Collection.PlayerFX_Collection" "DamageVignetteRadius" _vignetteradius :!class /Script/Engine.KismetMaterialLibrary))))

(event Custom|PlayShieldPP
  (bind (_direction _vigneteopacity _vignetteradius) (Timeline|Timeline_0 PlayFromStart)
    (:Update
      (Rendering|Material|SetScalarParameterValue "/Game/Materials/PlayerFX_Collection.PlayerFX_Collection" "ShieldVignetteOpacity" _vigneteopacity :!class /Script/Engine.KismetMaterialLibrary)
      (Rendering|Material|SetScalarParameterValue "/Game/Materials/PlayerFX_Collection.PlayerFX_Collection" "ShieldVignetteRadius" _vignetteradius :!class /Script/Engine.KismetMaterialLibrary))))

(event Custom|StopShieldPP
  (Rendering|Material|SetScalarParameterValue "/Game/Materials/PlayerFX_Collection.PlayerFX_Collection" "ShieldVignetteOpacity" 0.0 :!class /Script/Engine.KismetMaterialLibrary)
  (bind (_direction _vigneteopacity _vignetteradius) (Timeline|Timeline_0 Stop)
    (:Update
      (Rendering|Material|SetScalarParameterValue "/Game/Materials/PlayerFX_Collection.PlayerFX_Collection" "ShieldVignetteOpacity" _vigneteopacity :!class /Script/Engine.KismetMaterialLibrary)
      (Rendering|Material|SetScalarParameterValue "/Game/Materials/PlayerFX_Collection.PlayerFX_Collection" "ShieldVignetteRadius" _vignetteradius :!class /Script/Engine.KismetMaterialLibrary))))

(event EventSpawnShieldBP
  (AddComponent|AddChildActorComponent false))

(event EventBeginPlay
  (if (Pawn|IsLocallyControlled)
    (bind _returnvalue (UserInterface|CreateWidget "/Game/UI/AbilityMenu.AbilityMenu_C"))
    (Variables|Default|SetAbilityMenu _returnvalue)
    (else
      ;[1 1 1] Remove cockpit elements for non-locally controller players
      (Components|DestroyComponent (Variables|Default|GetRightHUD))
      (Components|DestroyComponent (Variables|Default|GetLeftHUD))
      (Components|DestroyComponent (Variables|Default|GetTopHUD))
      (Components|DestroyComponent (Variables|Default|GethulagirlPivot))
      (Components|DestroyComponent (Variables|Default|GetMiddleHUD))
      (Components|DestroyComponent (Variables|Default|GetAttackUpgradeButton))
      (Components|DestroyComponent (Variables|Default|GetDefenseUpgradeButton))
      (Components|DestroyComponent (Variables|Default|GetMobilityUpgradeButton))
      (Components|DestroyComponent (Variables|Default|GetAbilityMenuButton))
      (Components|DestroyComponent (Variables|Default|GetWindowUpper))
      (Components|DestroyComponent (Variables|Default|GetWindowTopBar))
      (Components|DestroyComponent (Variables|Default|GetWindowLower))
      (Components|DestroyComponent (Variables|Default|GetRaptor))
      (Components|DestroyComponent (Variables|Default|GetCow)))))

(event EventDieBP
  (Game|SpawnActorfromClass "/Game/Blueprints/Spawnable/ResourceOrbBP.ResourceOrbBP_C" (Math|Conversions|ToTransform(Vector) (Transformation|GetActorLocation)) "AdjustIfPossibleButAlwaysSpawn" self 0))

(event EventTick
  (params (DeltaSeconds :type Float%20%28single-precision%29))
  (if (Pawn|IsLocallyControlled)
    (Transformation|AddLocalRotation (Variables|Default|GethulagirlPivot) "0,1.000000, 0" false false)))

(event EventOpenAbilityMenuBP
  (UserInterface|Viewport|AddtoViewport (Variables|Default|GetAbilityMenu) 0))

(event EventCloseAbilityMenuBP
  (Widget|RemovefromParent (Variables|Default|GetAbilityMenu)))

(event EventTakeDamageBP
  (params (damage :type Integer) (damageType :type String))
  (CallFunction|ScreenShake))

(event EventShootBP
  (CallFunction|BroadcastPlaySound))

(event Game|Damage|EventAnyDamage
  (params (Damage :type Float%20%28single-precision%29) (DamageType :type Damage%20Type%20Object%20Reference) (InstigatedBy :type Controller%20Object%20Reference) (DamageCauser :type Actor%20Object%20Reference))
  (CallFunction|PlayPP))

(event Input|KeyboardEvents|T
  (params (Key :type Key%20Structure))
  (:Pressed
    (Rendering|SetVisibility (Variables|Default|GetRaptor) false false)
    (Rendering|SetVisibility (Variables|Default|GetCow) true false)))

(event Input|KeyboardEvents|R
  (params (Key :type Key%20Structure))
  (:Pressed
    (Rendering|SetVisibility (Variables|Default|GetCow) false false)
    (Rendering|SetVisibility (Variables|Default|GetRaptor) true false)))

(event Input|KeyboardEvents|LeftCtrl
  (params (Key :type Key%20Structure))
  (:Pressed
    ;[1 1 1] Enable Shield Vignete
    (bind (_direction _vigneteopacity _vignetteradius) (Timeline|Timeline_1 PlayFromStart)
      (:Update
        (Rendering|Material|SetScalarParameterValue "/Game/Materials/PlayerFX_Collection.PlayerFX_Collection" "DamageVignetteOpacity" _vigneteopacity :!class /Script/Engine.KismetMaterialLibrary)
        (Rendering|Material|SetScalarParameterValue "/Game/Materials/PlayerFX_Collection.PlayerFX_Collection" "DamageVignetteRadius" _vignetteradius :!class /Script/Engine.KismetMaterialLibrary)))))

(fn ConstructionScript)