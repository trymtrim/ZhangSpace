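; Container2 is an actor that removes itself when it strays extremely far from the world origin.
; Each tick, on the server only, it checks the absolute X, Y and Z of its location against a large bound and destroys itself if any axis reaches it.
; The construction script is empty and no other behavior is defined in the graphs.
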(event EventTick
  (params (DeltaSeconds :type Float%20%28single-precision%29))
  (bind _returnvalue (Transformation|GetActorLocation))
  (bind (_x _y _z) (Math|Vector|BreakVector _returnvalue))
  (if (Networking|IsServer)
    (if (Math|Boolean|ORBoolean (>= (Math|Float|Absolute(Float) _x) 1e+06) (>= (Math|Float|Absolute(Float) _y) 1e+06) (>= (Math|Float|Absolute(Float) _z) 1e+06))
      (Actor|DestroyActor))))

(fn ConstructionScript)