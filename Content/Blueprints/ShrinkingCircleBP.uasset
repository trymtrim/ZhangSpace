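; Shrinking circle actor that drives the visual blend of its Sphere material; the scaling of the sphere itself is not done here.
; BeginPlay sets a wide Blend Distance, waits, then a timeline lerps it toward a fraction of the sphere's world X scale.
; When the timeline finishes it sets InsideCircle, and Tick then keeps Blend Distance proportional to the sphere's current scale.
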(event EventTick
  (params (DeltaSeconds :type Float%20%28single-precision%29))
  (bind _sphere (Variables|Default|GetSphere))
  (if (Variables|Default|GetInsideCircle)
    (Rendering|Material|SetScalarParameterValueonMaterials _sphere "Blend Distance" (/ (.X (Math|Vector|BreakVector (Transformation|GetWorldScale _sphere))) 3.5))))

(event EventBeginPlay
  (bind _sphere (Variables|Default|GetSphere))
  (Rendering|Material|SetScalarParameterValueonMaterials _sphere "Blend Distance" 7e+03)
  (Utilities|FlowControl|Delay 22.0)
  (bind _lerpcirclevisual (Timeline|Timeline_0 Play)
    (:Update
      (Rendering|Material|SetScalarParameterValueonMaterials _sphere "Blend Distance" (Math|Float|Lerp 7e+03 (/ (.X (Math|Vector|BreakVector (Transformation|GetWorldScale _sphere))) 3.5) _lerpcirclevisual)))
    (:Finished
      (Variables|Default|SetInsideCircle true))))

(fn ConstructionScript)