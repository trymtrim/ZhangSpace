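; ResourceShardBP is a spawnable resource shard that breaks down into a ResourceOrbBP pickup or drop.
; Each begin-overlap on its static mesh subtracts a fixed amount from Health, with no filter on the overlapping actor.
; When Health runs out, it spawns the orb at its location and destroys itself.
; All of this logic runs only on the server, behind authority and IsServer checks.
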(event OnComponentBeginOverlap(StaticMeshComponent)
  (params (OverlappedComponent :type Primitive%20Component%20Object%20Reference) (OtherActor :type Actor%20Object%20Reference) (OtherComp :type Primitive%20Component%20Object%20Reference) (OtherBodyIndex :type Integer) (bFromSweep :type Boolean) (SweepResult :type Hit%20Result%20Structure%20%28by%20ref%29))
  (Networking|SwitchHasAuthority
    (:Authority
      (if (Networking|IsServer)
        (Variables|Default|SetHealth (- (Variables|Default|GetHealth) 20))
        (if (<= (Variables|Default|GetHealth) 0)
          (Game|SpawnActorfromClass "/Game/Blueprints/Spawnable/ResourceOrbBP.ResourceOrbBP_C" (Math|Transform|MakeTransform (Transformation|GetActorLocation)) "AlwaysSpawn" 0 0)
          (Actor|DestroyActor))))))

(fn ConstructionScript)