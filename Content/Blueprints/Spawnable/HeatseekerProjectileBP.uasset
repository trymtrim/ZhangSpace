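; Heatseeking projectile that homes on a target component and damages players it hits.
; On the server, Tick aligns the actor to its velocity and sharply sets homing acceleration very high once close to the target, which is assigned outside this graph.
; Server-side mesh overlaps with non-owner Player-tagged components apply the configurable damage, trigger impact particles and sound through a broadcast event, then destroy the projectile.
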(event OnComponentBeginOverlap(StaticMesh)
  (params (OverlappedComponent :type Primitive%20Component%20Object%20Reference) (OtherActor :type Actor%20Object%20Reference) (OtherComp :type Primitive%20Component%20Object%20Reference) (OtherBodyIndex :type Integer) (bFromSweep :type Boolean) (SweepResult :type Hit%20Result%20Structure%20%28by%20ref%29))
  (if (Networking|IsServer)
    (if (Components|ComponentHasTag OtherComp "Player")
      (if (not (== OtherActor (Components|GetOwner)))
        (Game|Damage|ApplyDamage OtherActor (Math|Conversions|ToFloat(Integer) (Variables|Default|GetDamage)) 0 self)
        (CallFunction|BroadcastSpawnParticle)
        (Actor|DestroyActor)))))

(event Custom|BroadcastSpawnParticle
  (Effects|SpawnEmitteratLocation "/Game/FX/CharacterFX/Impact/BulletImpact_FX.BulletImpact_FX" (Transformation|GetActorLocation) "0, 0, 0" "10.000000,10.000000,10.000000")
  (Audio|SpawnSoundAttached "/Game/Audio/FX/BulletFXImpact02_Cue.BulletFXImpact02_Cue" (Variables|Default|GetAudio) "None" "0, 0, 0" "0, 0, 0" "KeepRelativeOffset" false 1.0 1.0 0.0 0 0))

(event EventTick
  (params (DeltaSeconds :type Float%20%28single-precision%29))
  (bind _homingprojectilemovement (Variables|Default|GetHomingProjectileMovement))
  (if (Networking|IsServer)
    (Transformation|SetActorRotation (Math|Conversions|RotationFromXVector (Math|Vector|GetForwardVector (Math|Conversions|RotationFromXVector (Transformation|GetVelocity)))))
    (if (<= (Math|Vector|VectorLength (- (Transformation|GetActorLocation) (Transformation|GetWorldLocation (Variables|/Script/Engine.ProjectileMovementComponent|GetHomingTargetComponent _homingprojectilemovement)))) 5e+01)
      (Variables|/Script/Engine.ProjectileMovementComponent|SetHomingAccelerationMagnitude _homingprojectilemovement 4e+04))))

(fn ConstructionScript)

(fn SetDamage
  (params (Damage :type Integer))
  (Variables|Default|SetDamage Damage))