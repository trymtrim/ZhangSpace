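; Networked projectile fired by spaceships and other owners, optionally homing on a FollowTarget by re-aiming every server tick.
; The server sets launch velocity, using a fixed speed for SpaceshipAI owners and max speed otherwise, then enables hits.
; Authority-side sphere overlaps use component tags to damage players, AI and shields while ignoring the owner's own.
; Impacts broadcast a particle effect, with a sound for player hits, and destroy the projectile.
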(event OnComponentBeginOverlap(Sphere)
  (params (OverlappedComponent :type Primitive%20Component%20Object%20Reference) (OtherActor :type Actor%20Object%20Reference) (OtherComp :type Primitive%20Component%20Object%20Reference) (OtherBodyIndex :type Integer) (bFromSweep :type Boolean) (SweepResult :type Hit%20Result%20Structure%20%28by%20ref%29))
  (bind _damage (Variables|Default|Getdamage))
  (if (Variables|Default|GetCanHit)
    (Networking|SwitchHasAuthority
      (:Authority
        (if (Networking|IsServer)
          (if (Utilities|IsValid OtherComp)
            (if (or (Components|ComponentHasTag OtherComp "Player") (Components|ComponentHasTag OtherComp "AI"))
              (if (not (== OtherActor (Components|GetOwner)))
                (if (!= _damage 0.0)
                  (Game|Damage|ApplyDamage OtherActor _damage 0 self)
                  (CallFunction|BroadcastSpawnParticle)
                  (Actor|DestroyActor :!label _label)))
              (elif (Components|ComponentHasTag OtherComp "Shield")
                (if (not (== (Components|GetOwner) (Actor|GetParentActor OtherActor)))
                  (Game|Damage|ApplyDamage OtherActor (Variables|Default|Getdamage) 0 self)
                  (CallFunction|BroadcastSpawnParticle :!label _label_2)
                  (goto _label))
                (elif (not (== (Actor|GetParentActor OtherActor) (Components|GetOwner)))
                  (goto _label_2))))))))))

(event Custom|BroadcastSpawnParticle
  (Effects|SpawnEmitteratLocation "/Game/FX/CharacterFX/Impact/BulletImpact_FX.BulletImpact_FX" (Transformation|GetActorLocation))
  (if (Utilities|IsValid (stale OnComponentBeginOverlap(Sphere) OtherActor))
    (if (Components|ComponentHasTag (stale OnComponentBeginOverlap(Sphere) OtherComp) "Player")
      (Audio|SpawnSoundAttached "/Game/Audio/FX/BulletFXImpact02_Cue.BulletFXImpact02_Cue" (Variables|Default|GetAudio) "None" "0, 0, 0" "0, 0, 0" "KeepRelativeOffset" false 1.0 1.0 0.0 0 0))))

(event EventBeginPlay
  (bind _projectilemovement (Variables|Default|GetProjectileMovement))
  (Variables|Default|SetRotation (Transformation|GetActorRotation))
  (if (Networking|IsServer)
    (Utilities|FlowControl|Delay 0.0)
    (if (Utilities|ClassIsChildOf (Utilities|GetClass (Components|GetOwner)) "/Script/ZhangSpace.SpaceshipAI")
      (Variables|/Script/Engine.MovementComponent|SetVelocity _projectilemovement (* (Transformation|GetActorForwardVector) 2e+04))
      (else
        (Variables|/Script/Engine.MovementComponent|SetVelocity _projectilemovement (* (Transformation|GetActorForwardVector) (Variables|/Script/Engine.ProjectileMovementComponent|GetMaxSpeed _projectilemovement)))))
    (Variables|Default|SetCanHit true)))

(event EventTick
  (params (DeltaSeconds :type Float%20%28single-precision%29))
  (bind _projectilemovement (Variables|Default|GetProjectileMovement))
  (bind _followtarget (Variables|Default|GetfollowTarget))
  (if (Networking|IsServer)
    (if (Utilities|IsValid _followtarget)
      (Transformation|SetActorRotation (Math|Rotator|FindLookatRotation (Transformation|GetActorLocation) (Transformation|GetActorLocation _followtarget)))
      (Variables|/Script/Engine.MovementComponent|SetVelocity _projectilemovement (* (Transformation|GetActorForwardVector) (Variables|/Script/Engine.ProjectileMovementComponent|GetMaxSpeed _projectilemovement))))))

(fn ConstructionScript)