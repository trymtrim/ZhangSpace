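; Trap shot actor that bursts into a TrapFieldBP at its location and then destroys itself.
; The server triggers the burst after a short timed delay or on overlap, ignoring player components of its owner.
; Both triggers broadcast impact particles and sound and start the PlayerCharacter's trap shot cooldown.
; Detonate also bursts it but skips the cooldown call and server check; SetDamage is an empty stub.
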(event OnComponentBeginOverlap(StaticMesh)
  (params (OverlappedComponent :type Primitive%20Component%20Object%20Reference) (OtherActor :type Actor%20Object%20Reference) (OtherComp :type Primitive%20Component%20Object%20Reference) (OtherBodyIndex :type Integer) (bFromSweep :type Boolean) (SweepResult :type Hit%20Result%20Structure%20%28by%20ref%29))
  (if (Networking|IsServer)
    (if (Components|ComponentHasTag OtherComp "Player")
      (if (not (== OtherActor (Components|GetOwner)))
        (CallFunction|BroadcastSpawnParticle :!label _label)
        (Class|MainCharacterController|StartTrapShotCooldown (Variables|Default|GetPlayerCharacter))
        (Game|SpawnActorfromClass "/Game/Blueprints/Spawnable/TrapFieldBP.TrapFieldBP_C" (Math|Conversions|ToTransform(Vector) (Transformation|GetActorLocation)) "Undefined" 0 0)
        (Actor|DestroyActor))
      (else
        (goto _label)))))

(event Custom|BroadcastSpawnParticle
  (Effects|SpawnEmitteratLocation "/Game/FX/CharacterFX/Impact/BulletImpact_FX.BulletImpact_FX" (Transformation|GetActorLocation) "0, 0, 0" "10.000000,10.000000,10.000000")
  (Audio|SpawnSoundAttached "/Game/Audio/FX/BulletFXImpact02_Cue.BulletFXImpact02_Cue" (Variables|Default|GetAudio) "None" "0, 0, 0" "0, 0, 0" "KeepRelativeOffset" false 1.0 1.0 0.0 0 0))

(event Custom|Detonate
  (CallFunction|BroadcastSpawnParticle)
  (Game|SpawnActorfromClass "/Game/Blueprints/Spawnable/TrapFieldBP.TrapFieldBP_C" (Math|Conversions|ToTransform(Vector) (Transformation|GetActorLocation)) "Undefined" 0 0)
  (Actor|DestroyActor))

(event EventBeginPlay
  (if (Networking|IsServer)
    (Utilities|FlowControl|Delay 2.0)
    (CallFunction|BroadcastSpawnParticle)
    (Class|MainCharacterController|StartTrapShotCooldown (Variables|Default|GetPlayerCharacter))
    (Game|SpawnActorfromClass "/Game/Blueprints/Spawnable/TrapFieldBP.TrapFieldBP_C" (Math|Conversions|ToTransform(Vector) (Transformation|GetActorLocation)) "Undefined" 0 0)
    (Actor|DestroyActor)))

(fn ConstructionScript)

(fn SetDamage
  (params (Damage :type Integer)))