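; TeleporterBP is a spawnable teleporter that moves players who overlap its Cube component and displays as a wormhole.
; On overlap, only the server acts, calling TeleportPlayer on the overlapping actor when the touching component is tagged "Player".
; At BeginPlay it writes the Cube's world location into the WormholeCollection material parameter collection, so materials can read the wormhole's position.
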(event OnComponentBeginOverlap(Cube)
  (params (OverlappedComponent :type Primitive%20Component%20Object%20Reference) (OtherActor :type Actor%20Object%20Reference) (OtherComp :type Primitive%20Component%20Object%20Reference) (OtherBodyIndex :type Integer) (bFromSweep :type Boolean) (SweepResult :type Hit%20Result%20Structure%20%28by%20ref%29))
  (Networking|SwitchHasAuthority
    (:Authority
      (if (Networking|IsServer)
        (if (Utilities|IsValid OtherComp)
          (if (Components|ComponentHasTag OtherComp "Player")
            (Class|Teleporter|TeleportPlayer OtherActor)))))))

(event EventBeginPlay
  (Rendering|Material|SetVectorParameterValue "/Game/FX/CharacterFX/Wormhole/WormholeCollection.WormholeCollection" "Position" (Math|Conversions|ToLinearColor(Vector) (Transformation|GetWorldLocation (Variables|Default|GetCube))) :!class /Script/Engine.KismetMaterialLibrary))

(fn ConstructionScript)