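; TrapFieldBP is a spawnable, short-lived trap field actor that uses slow-field activation and deactivation sounds.
; On BeginPlay the server waits a fixed lifetime, then calls DestroyField and destroys the actor.
; Non-server instances play the attached activation cue, then stop it just before that lifetime ends and play the deactivation cue at the actor's location.
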(event EventBeginPlay
  (if (Networking|IsServer)
    (Utilities|FlowControl|Delay 1e+01)
    (Class|TrapShot|DestroyField)
    (Actor|DestroyActor)
    (else
      (bind _returnvalue (Audio|SpawnSoundAttached "/Game/Audio/FX/SlowFieldFXActivated_Cue.SlowFieldFXActivated_Cue" (Variables|Default|GetAudio) "None" "0, 0, 0" "0, 0, 0" "KeepRelativeOffset" false 1.0 1.0 0.0 0 0))
      (Utilities|FlowControl|Delay 9.75)
      (Audio|Components|Audio|Stop _returnvalue)
      (Audio|SpawnSoundatLocation "/Game/Audio/FX/SlowFieldFXDeactivated_Cue.SlowFieldFXDeactivated_Cue" (Transformation|GetActorLocation) "0, 0, 0" 1.0 1.0 0.0 0 0))))

(fn ConstructionScript)