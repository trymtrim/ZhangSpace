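; ResourceOrbBP is a replicated-game pickup orb that grants experience to player characters other than its owner.
; On an authoritative server overlap with a Player-tagged component, it adds experience to the MainCharacterController, triggers that player's client gain effect, and destroys itself.
; On BeginPlay, clients hide the mesh and particles if their local character owns the orb, so owners neither see nor collect it.
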(event OnComponentBeginOverlap(StaticMeshComponent)
  (params (OverlappedComponent :type Primitive%20Component%20Object%20Reference) (OtherActor :type Actor%20Object%20Reference) (OtherComp :type Primitive%20Component%20Object%20Reference) (OtherBodyIndex :type Integer) (bFromSweep :type Boolean) (SweepResult :type Hit%20Result%20Structure%20%28by%20ref%29))
  (Networking|SwitchHasAuthority
    (:Authority
      (if (Networking|IsServer)
        (if (Utilities|IsValid OtherComp)
          (if (Components|ComponentHasTag OtherComp "Player")
            (if (not (== (Components|GetOwner) OtherActor))
              (bind _asmain_character_controller (Utilities|Casting|CastToMainCharacterController OtherActor))
              (Class|MainCharacterController|AddExperience _asmain_character_controller (Variables|Default|GetExperience))
              (bind _asmain_character_controller_2 (Utilities|Casting|CastToMainCharacterController OtherActor))
              (Default|ClientExperienceGainEffect _asmain_character_controller_2)
              (Actor|DestroyActor))))))))

(event EventBeginPlay
  (if (not (Networking|IsServer))
    (if (== (Components|GetOwner) (Game|GetPlayerCharacter 0))
      (Rendering|SetVisibility (Variables|Default|GetParticleSystem) false false)
      (Rendering|SetVisibility (Variables|Debug|GetStaticMeshComponent) false false))))

(fn ConstructionScript)